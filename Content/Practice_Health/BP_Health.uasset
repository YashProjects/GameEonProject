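; BP_Health is a practice Blueprint that tracks an integer health value, HealthC, and prints changes to screen.
; The HealthReduce event subtracts a fixed amount, then either caps the value at an upper limit or prints it.
; AnyDamage sets HealthC to incoming damage minus current health, truncated, an operand order that is the reverse of usual damage subtraction, then prints it.
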(event `self.ReceiveBeginPlay`)

(event `/Game/BP_Interface/BPI_Health.HealthReduce`
  (bind _output_get (set `self.Health_C` (- (`self.Health_C`) 20)))
  (if (> (`self.Health_C`) 100)
    (set `self.Health_C` 100)
    (else
      (`KismetSystemLibrary.PrintString` (`KismetStringLibrary.Conv_IntToString` _output_get)))))

(event `self.ReceiveActorBeginOverlap`
  (params (OtherActor :type "Actor Object Reference")))

(event `self.ReceiveAnyDamage`
  (params (Damage :type "Float (single-precision)") (DamageType :type "DamageType Object Reference") (InstigatedBy :type "Controller Object Reference") (DamageCauser :type "Actor Object Reference"))
  (bind _output_get (set `self.Health_C` (`KismetMathLibrary.FTrunc` (- Damage (`KismetMathLibrary.Conv_IntToDouble` (`self.Health_C`))))))
  (`KismetSystemLibrary.PrintString` (`KismetStringLibrary.Conv_IntToString` _output_get)))

(fn `UserConstructionScript`)