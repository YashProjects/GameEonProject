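; BP_HeadGun is a socket-mounted gun turret that fires while valid and equipped, with magazine and reserve ammo.
; Fire spawns a muzzle flash and projectile, then updates ammo and its UI_WeaponSelection widget.
; Damage comes from a separate camera line trace, raised at its end, that sends health messages to the hit actor.
; AmmoCountFunc auto-refills an empty magazine from reserve, except when exactly 30 rounds remain there.
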(event `self.ReceiveBeginPlay`
  ;[1 1 1] Attach Turret to Actor
  (`SceneComponent.K2_AttachToComponent` (`self.Gun`) (`self.GunBase`) "Gun" "SnapToTarget" "SnapToTarget" "SnapToTarget" true)
  ;[1 1 1] Call UI For Ammo Update
  (bind _returnvalue (`|CreateWidget` "/Game/UI/UI_WeaponSelection.UI_WeaponSelection_C"))
  (set `self.UI_Weapon` _returnvalue))

(event `/Game/BP_Interface/BPI_Projectile.Fire`
  (params (`Is Valid` :type Boolean) (Equiped :type Boolean))
  (bind (_returnvalue_location _returnvalue_rotation _returnvalue_scale) (`KismetMathLibrary.BreakTransform` (`SceneComponent.K2_GetComponentToWorld` (`self.ProjectileLocation`))))
  (bind _playercameramanager (`PlayerController.PlayerCameraManager` (`GameplayStatics.GetPlayerController` 0)))
  (bind _returnvalue (`self.K2_GetActorLocation` _playercameramanager))
  ;[1 1 1] Fire Event
  (if (and `Is Valid` Equiped)
    (if (and (== (`self.AmmoHG`) 0) (== (`self.TotalAmmoHG`) 0))
      (`KismetSystemLibrary.PrintString` "No Ammo")
      (else
        (`GameplayStatics.SpawnEmitterAtLocation` "/Game/FXs/P_AssaultRifle_MF.P_AssaultRifle_MF" _returnvalue_location _returnvalue_rotation _returnvalue_scale)
        (`|SpawnActorFromClass` "/Game/Guns/Projectile/BP_HGProjectile.BP_HGProjectile_C" (`SceneComponent.K2_GetComponentToWorld` (`self.ProjectileLocation`)) "Undefined" "OverrideRootScale" null null)
        (`KismetSystemLibrary.PrintString` (`KismetStringLibrary.Concat_StrStr` (`KismetStringLibrary.Conv_IntToString` (`self.TotalAmmoHG`)) "/" (`KismetStringLibrary.Conv_IntToString` (`self.AmmoHG`))))
        (`self.Ammo Count Func`)
        (`/Game/BP_Interface/BPI_UI.Update Ammo` (`self.UI_Weapon`) (`self.TotalAmmoHG`) (`self.AmmoHG`))
        ;[1 1 1] Apply Damage
        (bind (_outhit _returnvalue_2) (`KismetSystemLibrary.LineTraceSingle` _returnvalue (`KismetMathLibrary.MakeVector` (.x (+ (* (`self.GetActorForwardVector` _playercameramanager) 2500.0) _returnvalue)) (.y (+ (* (`self.GetActorForwardVector` _playercameramanager) 2500.0) _returnvalue)) (+ (.z (+ (* (`self.GetActorForwardVector` _playercameramanager) 2500.0) _returnvalue)) 350.0)) "TraceTypeQuery1" false (`|MakeArray` self (`GameplayStatics.GetPlayerPawn` 0) (`GameplayStatics.GetPlayerController` 0) :!type "Actor Object Reference") "ForDuration"))
        (if _returnvalue_2
          (bind (_bblockinghit _binitialoverlap _time _distance _location _impactpoint _normal _impactnormal _physmat _hitactor) (`GameplayStatics.BreakHitResult` _outhit))
          (`KismetSystemLibrary.PrintString` (`KismetSystemLibrary.GetDisplayName` _hitactor))
          (message `/Game/BP_Interface/BPI_Health.HealthReduce` _hitactor)
          (message `/Game/BP_Interface/BPI_AIHealth.Damage Health` _hitactor))))))

(fn `Ammo Count Func`
  (set `self.AmmoHG` (- (`self.AmmoHG`) 1))
  (if (and (== (`self.AmmoHG`) 0) (> (`self.TotalAmmoHG`) 0))
    (if (< (`self.TotalAmmoHG`) 30)
      (set `self.AmmoHG` (`self.TotalAmmoHG`))
      (set `self.TotalAmmoHG` 0)
      (if (and (== (`self.AmmoHG`) 0) (== (`self.TotalAmmoHG`) 0))
        (set `self.AmmoHG` 0)
        (set `self.TotalAmmoHG` 0)
        (`KismetSystemLibrary.PrintString` "No Ammo"))
      (elif (> (`self.TotalAmmoHG`) 30)
        (bind _output_get (set `self.AmmoHG` 30))
        (set `self.TotalAmmoHG` (- (`self.TotalAmmoHG`) _output_get))))))

(fn `UserConstructionScript`)