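; Minigun weapon Blueprint that, when fired while valid and equipped, spawns four BP_HGProjectile actors and a muzzle flash.
; Each shot briefly scales a hidden capsule into a long hit volume, sending DamageHealthMessage to any actor that begins overlapping it.
; AmmoCountFunc decrements the magazine per shot and auto-refills it from reserve ammo in clips of up to 50, with ammo status printed on screen.
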(event `/Game/BP_Interface/BPI_Projectile.Fire`
  (params (`Is Valid` :type Boolean) (Equiped :type Boolean))
  (bind (_returnvalue_location _returnvalue_rotation _returnvalue_scale) (`KismetMathLibrary.BreakTransform` (`SceneComponent.K2_GetComponentToWorld` (`self.ProjectileLocation`))))
  ;[1 1 1] Fire
  (if (and `Is Valid` Equiped)
    (if (and (<= (`self.AmmoMG`) 0) (<= (`self.TotalAmmoMG`) 0))
      (`KismetSystemLibrary.PrintString` "No Ammo In MiniGun")
      (else
        (`self.Spawn Projectile`)
        (`GameplayStatics.SpawnEmitterAtLocation` "/Game/FXs/P_AssaultRifle_MF.P_AssaultRifle_MF" _returnvalue_location _returnvalue_rotation _returnvalue_scale)
        (`self.Ammo Count Func`)
        (`KismetSystemLibrary.PrintString` (`KismetStringLibrary.Concat_StrStr` (`KismetStringLibrary.Conv_IntToString` (`self.TotalAmmoMG`)) "/" (`KismetStringLibrary.Conv_IntToString` (`self.AmmoMG`))))
        (`SceneComponent.SetWorldScale3D` (`self.Capsule`) (0.5 0.5 29.5))
        (`KismetSystemLibrary.Delay` 0.1)
        (`SceneComponent.SetWorldScale3D` (`self.Capsule`) (0.0 0.0 0.0))))))

(event `self.ReceiveBeginPlay`
  (`SceneComponent.SetWorldScale3D` (`self.Capsule`) (0.0 0.0 0.0)))

(event `self.Capsule.OnComponentEndOverlap`
  (params (OverlappedComponent :type "PrimitiveComponent Object Reference") (OtherActor :type "Actor Object Reference") (OtherComp :type "PrimitiveComponent Object Reference") (OtherBodyIndex :type Integer))
  (cast `/Game/AI/BP_AICar` OtherActor)
  (set `self.Call` false))

(event `self.Capsule.OnComponentBeginOverlap`
  (params (OverlappedComponent :type "PrimitiveComponent Object Reference") (OtherActor :type "Actor Object Reference") (OtherComp :type "PrimitiveComponent Object Reference") (OtherBodyIndex :type Integer) (bFromSweep :type Boolean) (SweepResult :type "HitResult Structure (by ref)"))
  ;[1 1 1] Apply Damage (BPI - AI Damage Event)
  (set `self.Call` true)
  (if (`self.Call`)
    (message `/Game/BP_Interface/BPI_AIHealth.Damage Health` OtherActor)))

(event `self.Capsule.OnComponentHit`
  (params (HitComponent :type "PrimitiveComponent Object Reference") (OtherActor :type "Actor Object Reference") (OtherComp :type "PrimitiveComponent Object Reference") (NormalImpulse :type "Vector Structure") (Hit :type "HitResult Structure (by ref)"))
  (`KismetSystemLibrary.PrintString` (`KismetSystemLibrary.GetDisplayName` OtherActor)))

(fn `Ammo Count Func`
  ;[1 1 1] Ammo Count Func
  (set `self.AmmoMG` (- (`self.AmmoMG`) 1))
  (if (and (== (`self.AmmoMG`) 0) (> (`self.TotalAmmoMG`) 0))
    (if (< (`self.TotalAmmoMG`) 50)
      (set `self.AmmoMG` (`self.TotalAmmoMG`))
      (set `self.TotalAmmoMG` 0)
      (if (and (<= (`self.AmmoMG`) 0) (== (`self.TotalAmmoMG`) 0))
        (set `self.AmmoMG` 0)
        (set `self.TotalAmmoMG` 0)
        (`KismetSystemLibrary.PrintString` "No Ammo"))
      (elif (> (`self.TotalAmmoMG`) 50)
        (bind _output_get (set `self.AmmoMG` 50))
        (set `self.TotalAmmoMG` (- (`self.TotalAmmoMG`) _output_get))
        (elif (== (`self.TotalAmmoMG`) 50)
          (set `self.TotalAmmoMG` 0)
          (set `self.AmmoMG` 50))))))

(fn `Spawn Projectile`
  (`|SpawnActorFromClass` "/Game/Guns/Projectile/BP_HGProjectile.BP_HGProjectile_C" (`SceneComponent.K2_GetComponentToWorld` (`self.Location 4`)) "Undefined" "OverrideRootScale" null null)
  (`|SpawnActorFromClass` "/Game/Guns/Projectile/BP_HGProjectile.BP_HGProjectile_C" (`SceneComponent.K2_GetComponentToWorld` (`self.Location 1`)) "Undefined" "OverrideRootScale" null null)
  (`|SpawnActorFromClass` "/Game/Guns/Projectile/BP_HGProjectile.BP_HGProjectile_C" (`SceneComponent.K2_GetComponentToWorld` (`self.Location 2`)) "Undefined" "OverrideRootScale" null null)
  (`|SpawnActorFromClass` "/Game/Guns/Projectile/BP_HGProjectile.BP_HGProjectile_C" (`SceneComponent.K2_GetComponentToWorld` (`self.Location 3`)) "Undefined" "OverrideRootScale" null null)
  (return))

(fn `UserConstructionScript`)