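; BP_Missile is a homing missile that seeks a nearby target as soon as it spawns.
; BeginPlay runs a multi-sphere object trace around the missile, then turns and moves the mesh to a hit actor's sampled location with MoveComponentTo, without continuous tracking.
; After a delay it destroys itself, so the following delayed target destruction likely never fires.
; With nothing in range, it prints a message and self-destructs.
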(event EventBeginPlay
  (bind _missile (Variables|Default|GetMissile))
  (bind _returnvalue (Transformation|GetWorldLocation _missile))
  ;[1 1 1] Sphere Trace
  (bind _returnvalue_2 (Actor|GetActorOfClass "BP_Missile_C"))
  (bind (_outhits _returnvalue_3) (Collision|MultiSphereTraceForObjects _returnvalue _returnvalue 1e+03 (Utilities|Array|MakeArray "ObjectTypeQuery5" "ObjectTypeQuery3" "ObjectTypeQuery4") true (Utilities|Array|MakeArray (Game|GetPlayerController 0) self _returnvalue_2 (Game|Player|GetPlayerPawn 0) 0) "ForDuration"))
  (if _returnvalue_3
    ;[1 1 1] Missile Move To Target
    (Development|PrintString (Utilities|GetDisplayName (.hitactor (stale _array_element))))
    (Transformation|SetRelativeRotation (Variables|Default|GetMissile) (Math|Rotator|FindLookatRotation (Transformation|GetWorldLocation (Variables|Default|GetMissile)) (Transformation|GetActorLocation (.hitactor (stale _array_element)))) false false)
    (Variables|Default|SetTarget%20Location (Transformation|GetActorLocation (.hitactor (stale _array_element))))
    (Components|MoveComponentTo (Variables|Default|GetMissile) (Variables|Default|GetTarget%20Location) (Math|Rotator|FindLookatRotation (Transformation|GetWorldLocation (Variables|Default|GetMissile)) (Transformation|GetActorLocation (.hitactor (stale _array_element)))) false false 0.2 false)
    ;[1 1 1] Destroy Self & Target
    (Utilities|FlowControl|Delay 2.0)
    (Actor|DestroyActor)
    (Utilities|FlowControl|Delay 1.0)
    (Actor|DestroyActor (.hitactor (stale _array_element)))
    (else
      ;[1 1 1] No Ammo
      (Development|PrintString "No One In range")
      (Actor|DestroyActor))))

(event Collision|EventActorBeginOverlap
  (params (OtherActor :type Actor%20Object%20Reference)))

(event EventTick
  (params (DeltaSeconds :type Float%20%28single-precision%29)))

(fn ConstructionScript)